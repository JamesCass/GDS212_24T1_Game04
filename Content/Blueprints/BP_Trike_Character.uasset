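; BP_Trike_Character is the player's flipbook-animated Trike character, with jumping, a time-based score and death handling.
; Tick picks the run, jump or death flipbook, and a DoOnce reset on landing limits jumping to once per airtime.
; BeginPlay hides the cursor, detaches the camera in world space, and starts a looping timer feeding score to the UI widget.
; PlayerDead shows the game-over widget, then pauses after a short delay.
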(event `self.ReceiveTick`
  (params (DeltaSeconds :type "Float (single-precision)"))
  (if (`self.isDead`)
    (`PaperFlipbookComponent.SetFlipbook` (`self.Sprite`) "/Game/Assets/Characters/Trike/FB_Trike_Death.FB_Trike_Death")
    (elif (`NavMovementComponent.IsFalling` (`self.CharacterMovement`))
      (`PaperFlipbookComponent.SetFlipbook` (`self.Sprite`) "/Game/Assets/Characters/Trike/FB_Trike_Jump_Rise.FB_Trike_Jump_Rise")
      (else
        (`PaperFlipbookComponent.SetFlipbook` (`self.Sprite`) "/Game/Assets/Characters/Trike/FB_Trike_Run.FB_Trike_Run")))))

(event `InputAction|Jump`
  (params (Key :type "Key Structure"))
  ;[1 1 1] Jump Controls
  (:`Pressed`
    (if (not (`self.isDead`))
      (`/Engine/EditorBlueprintResources/StandardMacros.DoOnce` false :!label _label
        (:`Completed`
          (`self.Jump`))))))

(event `self.OnLanded`
  (params (Hit :type "HitResult Structure (by ref)"))
  ;[1 1 1] Jump Controls
  (goto _label :!via `Reset`))

(event `self.ReceiveBeginPlay`
  ;[0 0 0] Set cursor game mode
  (set `PlayerController.bShowMouseCursor` false (`GameplayStatics.GetPlayerController` 0))
  ;[0 0 0] Handle Player Score
  (`SceneComponent.K2_DetachFromComponent` (`self.Camera`) "KeepWorld" "KeepWorld" "KeepWorld" true)
  (bind _returnvalue (`|CreateWidget` "/Game/Blueprints/BP_GaneUI.BP_GaneUI_C"))
  (bind _output_get (set `self.Score` _returnvalue))
  (`UserWidget.AddToViewport` _output_get 0)
  (`KismetSystemLibrary.K2_SetTimerDelegate` (delegate `UpdateScore`) 0.1 true))

(event `UpdateScore`
  ;[0 0 0] Handle Player Score
  (if (not (`self.isDead`))
    (bind _result (`/Engine/EditorBlueprintResources/StandardMacros.IncrementInt` (`self.ScoreInt`))
      (:`  `
        (`/Game/Blueprints/BP_GaneUI.UpdateScore` (`self.Score`) _result)))))

(event `PlayerDead`
  ;[0.4427 0.003741 0] PlayerDeath
  (set `self.isDead` true)
  (bind _returnvalue (`|CreateWidget` "/Game/Blueprints/BP_GameOver.BP_GameOver_C"))
  (`UserWidget.AddToViewport` _returnvalue 0)
  (`KismetSystemLibrary.Delay` 0.2)
  (`GameplayStatics.SetGamePaused` true))

(fn `UserConstructionScript`)