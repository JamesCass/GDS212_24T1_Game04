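; BP_FlyerSpawner is an endless-mode obstacle spawner that randomly spawns BP_Flyer actors at its Scene component's transform.
; BeginPlay starts a looping timer with a random interval, rolled once per spawner.
; Each tick of that timer makes a random roll to spawn, with the odds rising in stages as elapsed game time passes two thresholds.
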(event `self.ReceiveBeginPlay`
  (`KismetSystemLibrary.K2_SetTimerDelegate` (delegate `SpawnRandomFlyer`) (`KismetMathLibrary.RandomFloatInRange` 0.5 2.5) true))

(event `SpawnRandomFlyer`
  (if (>= (`GameplayStatics.GetTimeSeconds`) 20.0)
    (if (>= (`GameplayStatics.GetTimeSeconds`) 35.0)
      (switch `int` (`KismetMathLibrary.RandomIntegerInRange` 0 2)
        (:`0`
          (`|SpawnActorFromClass` "/Game/Blueprints/EndlessGameMode/Obstacles/BP_Flyer.BP_Flyer_C" (`SceneComponent.K2_GetComponentToWorld` (`self.Scene`)) "Undefined" "MultiplyWithRoot" null null)))
      (else
        (switch `int` (`KismetMathLibrary.RandomIntegerInRange` 0 3)
          (:`0`
            (`|SpawnActorFromClass` "/Game/Blueprints/EndlessGameMode/Obstacles/BP_Flyer.BP_Flyer_C" (`SceneComponent.K2_GetComponentToWorld` (`self.Scene`)) "Undefined" "MultiplyWithRoot" null null)))))
    (else
      (switch `int` (`KismetMathLibrary.RandomIntegerInRange` 0 4)
        (:`0`
          (`|SpawnActorFromClass` "/Game/Blueprints/EndlessGameMode/Obstacles/BP_Flyer.BP_Flyer_C" (`SceneComponent.K2_GetComponentToWorld` (`self.Scene`)) "Undefined" "MultiplyWithRoot" null null))))))

(fn `UserConstructionScript`)