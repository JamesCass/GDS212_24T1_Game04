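; Spawner actor for endless game mode that periodically creates random ground obstacles at its Scene component's transform.
; On BeginPlay it starts a looping timer whose interval is randomized once, between one and two seconds.
; Each tick of the timer rolls a random integer to pick a skull, rib cage, cactus, small mound or large mound.
; Only half of the possible rolls map to an obstacle, so the rest leave gaps.
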(event `self.ReceiveBeginPlay`
  (`KismetSystemLibrary.K2_SetTimerDelegate` (delegate `SpawnRandomObstacle`) (`KismetMathLibrary.RandomFloatInRange` 1.0 2.0) true))

(event `SpawnRandomObstacle`
  (switch `int` (`KismetMathLibrary.RandomIntegerInRange` 0 9)
    (:`0`
      (`|SpawnActorFromClass` "/Game/Blueprints/EndlessGameMode/Obstacles/BP_Skull.BP_Skull_C" (`SceneComponent.K2_GetComponentToWorld` (`self.Scene`)) "Undefined" "MultiplyWithRoot" null null))
    (:`1`
      (`|SpawnActorFromClass` "/Game/Blueprints/EndlessGameMode/Obstacles/BP_RibCage.BP_RibCage_C" (`SceneComponent.K2_GetComponentToWorld` (`self.Scene`)) "Undefined" "MultiplyWithRoot" null null))
    (:`2`
      (`|SpawnActorFromClass` "/Game/Blueprints/EndlessGameMode/Obstacles/BP_Cactus.BP_Cactus_C" (`SceneComponent.K2_GetComponentToWorld` (`self.Scene`)) "Undefined" "MultiplyWithRoot" null null))
    (:`3`
      (`|SpawnActorFromClass` "/Game/Blueprints/EndlessGameMode/Obstacles/BP_SmallMound.BP_SmallMound_C" (`SceneComponent.K2_GetComponentToWorld` (`self.Scene`)) "Undefined" "MultiplyWithRoot" null null))
    (:`4`
      (`|SpawnActorFromClass` "/Game/Blueprints/EndlessGameMode/Obstacles/BP_LargeMound.BP_LargeMound_C" (`SceneComponent.K2_GetComponentToWorld` (`self.Scene`)) "Undefined" "MultiplyWithRoot" null null))))

(fn `UserConstructionScript`)