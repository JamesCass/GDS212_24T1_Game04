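; Player character for an endless runner mode: a flipbook-animated Trike that can jump and slide (crouch) through Enhanced Input.
; BeginPlay detaches the camera in world space, adds the input mapping and score widget, and starts a looping timer that raises the score while alive.
; Tick picks the run, jump or hit flipbook from the death and falling states.
; PlayerDead shows the game over widget, then pauses the game after a short delay.
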(event `self.ReceiveTick`
  (params (DeltaSeconds :type "Float (single-precision)"))
  (if (`self.isDead`)
    (`PaperFlipbookComponent.SetFlipbook` (`self.Sprite`) "/Game/Assets/Characters/Trike/FB_Trike_Hit.FB_Trike_Hit")
    (elif (`NavMovementComponent.IsFalling` (`self.CharacterMovement`))
      (`PaperFlipbookComponent.SetFlipbook` (`self.Sprite`) "/Game/Assets/Characters/Trike/FB_Trike_Jump_Rise.FB_Trike_Jump_Rise")
      (else
        (`PaperFlipbookComponent.SetFlipbook` (`self.Sprite`) "/Game/Assets/Characters/Trike/FB_Trike_Run.FB_Trike_Run")))))

(event `self.ReceiveBeginPlay`
  (`|ExecutionSequence`
    (:`then_0`
      ;[0 0 0] Set cursor game mode
      (set `PlayerController.bShowMouseCursor` false (`GameplayStatics.GetPlayerController` 0))
      ;[0 0 0] Handle Player Score
      (`SceneComponent.K2_DetachFromComponent` (`self.Camera`) "KeepWorld" "KeepWorld" "KeepWorld" true)
      (bind _returnvalue (`|CreateWidget` "/Game/Blueprints/EndlessGameMode/BP_GaneUI.BP_GaneUI_C"))
      (bind _output_get (set `self.Score` _returnvalue))
      (`UserWidget.AddToViewport` _output_get 0)
      (`KismetSystemLibrary.K2_SetTimerDelegate` (delegate `UpdateScore`) 0.1 true))
    (:`then_1`
      (bind _asplayer_controller (cast `PlayerController` (`self.GetController`)))
      (`EnhancedInputSubsystemInterface.AddMappingContext` (pcsubsystem `EnhancedInputLocalPlayerSubsystem` _asplayer_controller) "/Game/Blueprints/EndlessGameMode/Input/IMC_Endless.IMC_Endless" 0 (struct)))))

(event `UpdateScore`
  ;[0 0 0] Handle Player Score
  (if (not (`self.isDead`))
    (bind _result (`/Engine/EditorBlueprintResources/StandardMacros.IncrementInt` (`self.ScoreInt`))
      (:`  `
        (`/Game/Blueprints/EndlessGameMode/BP_GaneUI.UpdateScore` (`self.Score`) _result)))))

(event `PlayerDead`
  ;[0.4427 0.003741 0] PlayerDeath
  (set `self.isDead` true)
  (bind _returnvalue (`|CreateWidget` "/Game/Blueprints/EndlessGameMode/BP_GameOver.BP_GameOver_C"))
  (`UserWidget.AddToViewport` _returnvalue 0)
  (`KismetSystemLibrary.Delay` 0.2)
  (`GameplayStatics.SetGamePaused` true))

(event `EnhancedInput|/Game/Blueprints/EndlessGameMode/Input/Actions/IA_Jump`
  (params (ActionValue :type Boolean) (ElapsedSeconds :type "Float (double-precision)") (TriggeredSeconds :type "Float (double-precision)") (InputAction :type "InputAction Object Reference" :default "/Game/Blueprints/EndlessGameMode/Input/Actions/IA_Jump.IA_Jump"))
  (:`Started`
    (if (not (`self.isDead`))
      (`self.Jump`)
      (`KismetSystemLibrary.PrintString` "Hello")))
  (:`Completed`
    (`self.StopJumping`)))

(event `EnhancedInput|/Game/Blueprints/EndlessGameMode/Input/Actions/IA_Slide`
  (params (ActionValue :type Boolean) (ElapsedSeconds :type "Float (double-precision)") (TriggeredSeconds :type "Float (double-precision)") (InputAction :type "InputAction Object Reference" :default "/Game/Blueprints/EndlessGameMode/Input/Actions/IA_Slide.IA_Slide"))
  (:`Started`
    (if (not (`self.isDead`))
      (`self.Crouch`)))
  (:`Completed`
    (`self.UnCrouch`)))

(fn `UserConstructionScript`)