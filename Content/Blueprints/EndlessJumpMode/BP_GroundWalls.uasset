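; BP_GroundWalls is an Endless Jump mode actor that wraps BP_Bronto_Character horizontally across the play area.
; Overlapping the left or right ScreenWrap collider teleports the character to the X position of the arrow component on the opposite side.
; Only X changes, so the character keeps its Y and height when crossing.
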(event `self.ScreenWrapLeft.OnComponentBeginOverlap`
  (params (OverlappedComponent :type "PrimitiveComponent Object Reference") (OtherActor :type "Actor Object Reference") (OtherComp :type "PrimitiveComponent Object Reference") (OtherBodyIndex :type Integer) (bFromSweep :type Boolean) (SweepResult :type "HitResult Structure (by ref)"))
  (bind _returnvalue_x (`KismetMathLibrary.BreakVector` (`SceneComponent.K2_GetComponentLocation` (`self.ArrowRight`))))
  ;[0 0 0] Teleport player to right side arrow when touching left collider
  (bind _asbp_bronto_character (cast `/Game/Blueprints/EndlessJumpMode/BP_Bronto_Character` OtherActor))
  (bind (_returnvalue_x_2 _returnvalue_y _returnvalue_z) (`KismetMathLibrary.BreakVector` (`self.K2_GetActorLocation` _asbp_bronto_character)))
  (`self.K2_SetActorLocation` _asbp_bronto_character (`KismetMathLibrary.MakeVector` _returnvalue_x _returnvalue_y _returnvalue_z) false true))

(event `self.ScreenWrapRight.OnComponentBeginOverlap`
  (params (OverlappedComponent :type "PrimitiveComponent Object Reference") (OtherActor :type "Actor Object Reference") (OtherComp :type "PrimitiveComponent Object Reference") (OtherBodyIndex :type Integer) (bFromSweep :type Boolean) (SweepResult :type "HitResult Structure (by ref)"))
  (bind _returnvalue_x (`KismetMathLibrary.BreakVector` (`SceneComponent.K2_GetComponentLocation` (`self.ArrowLeft`))))
  ;[0 0 0] Teleport player to left side arrow when touching right collider
  (bind _asbp_bronto_character (cast `/Game/Blueprints/EndlessJumpMode/BP_Bronto_Character` OtherActor))
  (bind (_returnvalue_x_2 _returnvalue_y _returnvalue_z) (`KismetMathLibrary.BreakVector` (`self.K2_GetActorLocation` _asbp_bronto_character)))
  (`self.K2_SetActorLocation` _asbp_bronto_character (`KismetMathLibrary.MakeVector` _returnvalue_x _returnvalue_y _returnvalue_z) false true))

(fn `UserConstructionScript`)