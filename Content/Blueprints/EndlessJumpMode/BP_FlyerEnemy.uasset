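; Flying enemy for the endless jump mode that kills the Bronto player character on contact.
; An overlap on FlyerCollider checks the character's vertical velocity.
; Both branches call PlayerDead on player character 0, but when the character is not moving upward, a zero LaunchCharacter with Z override first cancels its vertical velocity.
; The Blueprint's graphs contain no movement logic.
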(event `self.ReceiveTick`
  (params (DeltaSeconds :type "Float (single-precision)")))

(event `self.FlyerCollider.OnComponentBeginOverlap`
  (params (OverlappedComponent :type "PrimitiveComponent Object Reference") (OtherActor :type "Actor Object Reference") (OtherComp :type "PrimitiveComponent Object Reference") (OtherBodyIndex :type Integer) (bFromSweep :type Boolean) (SweepResult :type "HitResult Structure (by ref)"))
  (bind _asbp_bronto_character (cast `/Game/Blueprints/EndlessJumpMode/BP_Bronto_Character` OtherActor))
  (bind (_returnvalue_x _returnvalue_y _returnvalue_z) (`KismetMathLibrary.BreakVector` (`self.GetVelocity` _asbp_bronto_character)))
  (if (> _returnvalue_z 0.0)
    (bind _asbp_bronto_character_2 (cast `/Game/Blueprints/EndlessJumpMode/BP_Bronto_Character` (`GameplayStatics.GetPlayerCharacter` 0)))
    (`/Game/Blueprints/EndlessJumpMode/BP_Bronto_Character.PlayerDead` _asbp_bronto_character_2)
    (else
      (`Character.LaunchCharacter` _asbp_bronto_character (0.0 0.0 0.0) false true)
      (bind _asbp_bronto_character_3 (cast `/Game/Blueprints/EndlessJumpMode/BP_Bronto_Character` (`GameplayStatics.GetPlayerCharacter` 0)))
      (`/Game/Blueprints/EndlessJumpMode/BP_Bronto_Character.PlayerDead` _asbp_bronto_character_3))))

(fn `UserConstructionScript`)