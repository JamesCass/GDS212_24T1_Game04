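; Map segment for the endless jump mode that chains level generation and handles screen wrap and fall death.
; The construction script randomizes the relative Y position of three child-actor platforms.
; The player's first overlap with the generation trigger spawns a BP_Map at the next-spawn transform, then destroys the trigger.
; Side colliders teleport the player to the opposite arrow's X, and the death box kills the player only when falling fast.
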(event `self.PlatformGenerateCollision.OnComponentBeginOverlap`
  (params (OverlappedComponent :type "PrimitiveComponent Object Reference") (OtherActor :type "Actor Object Reference") (OtherComp :type "PrimitiveComponent Object Reference") (OtherBodyIndex :type Integer) (bFromSweep :type Boolean) (SweepResult :type "HitResult Structure (by ref)"))
  ;[0 0 0] When map gen collider is entered by the player spawn next map from array of 3 types then destroy collider to prevent extra spawns
  (`/Engine/EditorBlueprintResources/StandardMacros.DoOnce` false
    (:`Completed`
      (cast `/Game/Blueprints/EndlessJumpMode/BP_Bronto_Character` OtherActor)
      (`|SpawnActorFromClass` "/Game/Blueprints/EndlessJumpMode/BP_Map.BP_Map_C" (`SceneComponent.K2_GetComponentToWorld` (`self.NextSpawnLoaction`)) "Undefined" "MultiplyWithRoot" null null)
      (`ActorComponent.K2_DestroyComponent` (`self.PlatformGenerateCollision`)))))

(event `self.ScreenWrapLeft.OnComponentBeginOverlap`
  (params (OverlappedComponent :type "PrimitiveComponent Object Reference") (OtherActor :type "Actor Object Reference") (OtherComp :type "PrimitiveComponent Object Reference") (OtherBodyIndex :type Integer) (bFromSweep :type Boolean) (SweepResult :type "HitResult Structure (by ref)"))
  (bind _returnvalue_x (`KismetMathLibrary.BreakVector` (`SceneComponent.K2_GetComponentLocation` (`self.ArrowRight`))))
  ;[0 0 0] Teleport player to right side arrow when touching left collider
  (bind _asbp_bronto_character (cast `/Game/Blueprints/EndlessJumpMode/BP_Bronto_Character` OtherActor))
  (bind (_returnvalue_x_2 _returnvalue_y _returnvalue_z) (`KismetMathLibrary.BreakVector` (`self.K2_GetActorLocation` _asbp_bronto_character)))
  (`self.K2_SetActorLocation` _asbp_bronto_character (`KismetMathLibrary.MakeVector` _returnvalue_x _returnvalue_y _returnvalue_z) false true))

(event `self.ScreenWrapRight.OnComponentBeginOverlap`
  (params (OverlappedComponent :type "PrimitiveComponent Object Reference") (OtherActor :type "Actor Object Reference") (OtherComp :type "PrimitiveComponent Object Reference") (OtherBodyIndex :type Integer) (bFromSweep :type Boolean) (SweepResult :type "HitResult Structure (by ref)"))
  (bind _returnvalue_x (`KismetMathLibrary.BreakVector` (`SceneComponent.K2_GetComponentLocation` (`self.ArrowLeft`))))
  ;[0 0 0] Teleport player to left side arrow when touching right collider
  (bind _asbp_bronto_character (cast `/Game/Blueprints/EndlessJumpMode/BP_Bronto_Character` OtherActor))
  (bind (_returnvalue_x_2 _returnvalue_y _returnvalue_z) (`KismetMathLibrary.BreakVector` (`self.K2_GetActorLocation` _asbp_bronto_character)))
  (`self.K2_SetActorLocation` _asbp_bronto_character (`KismetMathLibrary.MakeVector` _returnvalue_x _returnvalue_y _returnvalue_z) false true))

(event `self.DeathBox.OnComponentBeginOverlap`
  (params (OverlappedComponent :type "PrimitiveComponent Object Reference") (OtherActor :type "Actor Object Reference") (OtherComp :type "PrimitiveComponent Object Reference") (OtherBodyIndex :type Integer) (bFromSweep :type Boolean) (SweepResult :type "HitResult Structure (by ref)"))
  ;[0 0 0] If player is going fast enough and collides with death box then set dead
  (bind _asbp_bronto_character (cast `/Game/Blueprints/EndlessJumpMode/BP_Bronto_Character` OtherActor))
  (bind (_returnvalue_x _returnvalue_y _returnvalue_z) (`KismetMathLibrary.BreakVector` (`self.GetVelocity` _asbp_bronto_character)))
  (if (not (> _returnvalue_z -2000.0))
    (`/Game/Blueprints/EndlessJumpMode/BP_Bronto_Character.PlayerDead` _asbp_bronto_character)))

(fn `UserConstructionScript`
  (bind _childactor2 (`self.ChildActor2`))
  (bind _childactor (`self.ChildActor`))
  (bind _childactor1 (`self.ChildActor1`))
  (bind (_relativelocation_x _relativelocation_y _relativelocation_z) (`KismetMathLibrary.BreakVector` (`SceneComponent.RelativeLocation` _childactor1)))
  (bind (_relativelocation_x_2 _relativelocation_y_2 _relativelocation_z_2) (`KismetMathLibrary.BreakVector` (`SceneComponent.RelativeLocation` _childactor2)))
  (bind (_relativelocation_x_3 _relativelocation_y_3 _relativelocation_z_3) (`KismetMathLibrary.BreakVector` (`SceneComponent.RelativeLocation` _childactor)))
  ;[0 0 0] Set location of platforms at random location on Y
  (`SceneComponent.K2_SetRelativeLocation` _childactor (`KismetMathLibrary.MakeVector` _relativelocation_x_3 (`KismetMathLibrary.RandomFloatInRange` -430.0 430.0) _relativelocation_z_3) false false)
  (`SceneComponent.K2_SetRelativeLocation` _childactor1 (`KismetMathLibrary.MakeVector` _relativelocation_x (`KismetMathLibrary.RandomFloatInRange` -430.0 430.0) _relativelocation_z) false false)
  (`SceneComponent.K2_SetRelativeLocation` _childactor2 (`KismetMathLibrary.MakeVector` _relativelocation_x_2 (`KismetMathLibrary.RandomFloatInRange` -430.0 430.0) _relativelocation_z_2) false false))