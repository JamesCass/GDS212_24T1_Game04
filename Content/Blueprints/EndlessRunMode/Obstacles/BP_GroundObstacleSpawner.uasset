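; Spawner for endless run mode that drops random ground obstacles (rib cage, cactus, mounds, skull) at its Scene component's transform.
; BeginPlay starts a looping timer whose interval is randomized only once, so each spawner keeps a fixed cadence.
; Each tick of that timer rolls a random integer where unmatched values spawn nothing.
; The roll range narrows at two world-time thresholds, raising spawn odds as the run progresses.
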(event `self.ReceiveBeginPlay`
  (`KismetSystemLibrary.K2_SetTimerDelegate` (delegate `SpawnRandomObstacle`) (`KismetMathLibrary.RandomFloatInRange` 1.0 2.0) true))

(event `SpawnRandomObstacle`
  (if (>= (`GameplayStatics.GetTimeSeconds`) 20.0)
    (if (>= (`GameplayStatics.GetTimeSeconds`) 35.0)
      ;[0 0 0] 5/6 chance to spawn obstacle after 35 seconds
      (switch `int` (`KismetMathLibrary.RandomIntegerInRange` 0 5)
        (:`1`
          (`|SpawnActorFromClass` "/Game/Blueprints/EndlessRunMode/Obstacles/BP_RibCage.BP_RibCage_C" (`SceneComponent.K2_GetComponentToWorld` (`self.Scene`)) "Undefined" "MultiplyWithRoot" null null))
        (:`2`
          (`|SpawnActorFromClass` "/Game/Blueprints/EndlessRunMode/Obstacles/BP_Cactus.BP_Cactus_C" (`SceneComponent.K2_GetComponentToWorld` (`self.Scene`)) "Undefined" "MultiplyWithRoot" null null))
        (:`3`
          (`|SpawnActorFromClass` "/Game/Blueprints/EndlessRunMode/Obstacles/BP_SmallMound.BP_SmallMound_C" (`SceneComponent.K2_GetComponentToWorld` (`self.Scene`)) "Undefined" "MultiplyWithRoot" null null))
        (:`4`
          (`|SpawnActorFromClass` "/Game/Blueprints/EndlessRunMode/Obstacles/BP_LargeMound.BP_LargeMound_C" (`SceneComponent.K2_GetComponentToWorld` (`self.Scene`)) "Undefined" "MultiplyWithRoot" null null))
        (:`5`
          (`|SpawnActorFromClass` "/Game/Blueprints/EndlessRunMode/Obstacles/BP_Skull.BP_Skull_C" (`SceneComponent.K2_GetComponentToWorld` (`self.Scene`)) "Undefined" "MultiplyWithRoot" null null)))
      (else
        ;[0 0 0] 5/7 chance to spawn obstacle after 20 seconds
        (switch `int` (`KismetMathLibrary.RandomIntegerInRange` 0 6)
          (:`1`
            (`|SpawnActorFromClass` "/Game/Blueprints/EndlessRunMode/Obstacles/BP_RibCage.BP_RibCage_C" (`SceneComponent.K2_GetComponentToWorld` (`self.Scene`)) "Undefined" "MultiplyWithRoot" null null))
          (:`2`
            (`|SpawnActorFromClass` "/Game/Blueprints/EndlessRunMode/Obstacles/BP_Cactus.BP_Cactus_C" (`SceneComponent.K2_GetComponentToWorld` (`self.Scene`)) "Undefined" "MultiplyWithRoot" null null))
          (:`3`
            (`|SpawnActorFromClass` "/Game/Blueprints/EndlessRunMode/Obstacles/BP_SmallMound.BP_SmallMound_C" (`SceneComponent.K2_GetComponentToWorld` (`self.Scene`)) "Undefined" "MultiplyWithRoot" null null))
          (:`4`
            (`|SpawnActorFromClass` "/Game/Blueprints/EndlessRunMode/Obstacles/BP_LargeMound.BP_LargeMound_C" (`SceneComponent.K2_GetComponentToWorld` (`self.Scene`)) "Undefined" "MultiplyWithRoot" null null))
          (:`5`
            (`|SpawnActorFromClass` "/Game/Blueprints/EndlessRunMode/Obstacles/BP_Skull.BP_Skull_C" (`SceneComponent.K2_GetComponentToWorld` (`self.Scene`)) "Undefined" "MultiplyWithRoot" null null)))))
    (else
      ;[0 0 0] 5/9 chance to spawn obstacle for first 20 seconds
      (switch `int` (`KismetMathLibrary.RandomIntegerInRange` 0 8)
        (:`1`
          (`|SpawnActorFromClass` "/Game/Blueprints/EndlessRunMode/Obstacles/BP_RibCage.BP_RibCage_C" (`SceneComponent.K2_GetComponentToWorld` (`self.Scene`)) "Undefined" "MultiplyWithRoot" null null))
        (:`2`
          (`|SpawnActorFromClass` "/Game/Blueprints/EndlessRunMode/Obstacles/BP_Cactus.BP_Cactus_C" (`SceneComponent.K2_GetComponentToWorld` (`self.Scene`)) "Undefined" "MultiplyWithRoot" null null))
        (:`3`
          (`|SpawnActorFromClass` "/Game/Blueprints/EndlessRunMode/Obstacles/BP_SmallMound.BP_SmallMound_C" (`SceneComponent.K2_GetComponentToWorld` (`self.Scene`)) "Undefined" "MultiplyWithRoot" null null))
        (:`4`
          (`|SpawnActorFromClass` "/Game/Blueprints/EndlessRunMode/Obstacles/BP_LargeMound.BP_LargeMound_C" (`SceneComponent.K2_GetComponentToWorld` (`self.Scene`)) "Undefined" "MultiplyWithRoot" null null))
        (:`5`
          (`|SpawnActorFromClass` "/Game/Blueprints/EndlessRunMode/Obstacles/BP_Skull.BP_Skull_C" (`SceneComponent.K2_GetComponentToWorld` (`self.Scene`)) "Undefined" "MultiplyWithRoot" null null))))))

(fn `UserConstructionScript`)